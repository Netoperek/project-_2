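; PB_WinVolume is a trigger volume that acts as the level's finish point for the player.
; When the player pawn overlaps it, an IsWin check picks the win or lose message and passes it to BP_PlayerPawn's Meta call with a display time.
; On a win it waits out that display time, then calls NextLevel with the configured Level; on a loss it only sends the message.
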(event Collision|EventActorBeginOverlap
  (params (OtherActor :type Actor%20Object%20Reference))
  (if (== OtherActor (Game|Player|GetPlayerPawn 0))
    (Utilities|IsWin
      (:True
        (bind _outactors (Actor|GetAllActorsOfClass "/Game/Blueprints/Actors/Pawn/BP_PlayerPawn.BP_PlayerPawn_C"))
        (Default|Meta (Utilities|Array|Get(acopy) _outactors) (Variables|Default|GetMessageWin) (Variables|Default|GetTime%20Show%20Message))
        (Utilities|FlowControl|Delay (Variables|Default|GetTime%20Show%20Message))
        (Utilities|NextLevel (Variables|Default|GetLevel)))
      (:False
        (bind _outactors_2 (Actor|GetAllActorsOfClass "/Game/Blueprints/Actors/Pawn/BP_PlayerPawn.BP_PlayerPawn_C"))
        (Default|Meta (Utilities|Array|Get(acopy) _outactors_2) (Variables|Default|GetMessageLose) (Variables|Default|GetTime%20Show%20Message))))))

(fn ConstructionScript)