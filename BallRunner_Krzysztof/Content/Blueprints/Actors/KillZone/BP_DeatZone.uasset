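; Kill zone actor that restarts the current level when the player pawn overlaps it.
; On overlap it fades the camera and audio to black, waits for the fade duration, then reopens the level by its current name.
; On BeginPlay it fades the camera back in from black, sharing the same duration variable, so the restart reads as one smooth transition.
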(event Collision|EventActorBeginOverlap
  (params (OtherActor :type Actor%20Object%20Reference))
  ;[1 1 1] Event Restart Level && Fade Camera
  (if (== OtherActor (Game|Player|GetPlayerPawn 0))
    (CameraFades|StartCameraFade (Game|GetPlayerCameraManager 0) 0.0 1.0 (Variables|Default|GetDurationTime) "(R=0.000000,G=0.000000,B=0.000000,A=1.000000)" true false)
    (Utilities|FlowControl|Delay (Variables|Default|GetDurationTime))
    (bind _returnvalue (Game|GetCurrentLevelName true))
    (Game|OpenLevel(byName) (Utilities|String|StringToName _returnvalue))))

(event EventBeginPlay
  ;[1 1 1] Start Fade Cmera
  (CameraFades|StartCameraFade (Game|GetPlayerCameraManager 0) 1.0 0.0 (Variables|Default|GetDurationTime) "(R=0.000000,G=0.000000,B=0.000000,A=1.000000)" true false))

(fn ConstructionScript)