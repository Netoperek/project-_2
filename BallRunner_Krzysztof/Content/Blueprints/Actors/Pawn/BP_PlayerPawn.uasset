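; BP_PlayerPawn is a rolling-ball player pawn that collects crystals and shows timed on-screen messages.
; Axis inputs apply torque to the Ball, while HitCrystal adds points toward a max score counted from BP_Crystal actors at BeginPlay.
; Meta briefly displays text on its UI_Messege widget, and KillPlayer fades the camera to black, then reloads the current level.
; The spring arm length is overridden on Level2.
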(event Custom|KillPlayer
  ;[1 1 1] Kill Player
  (CameraFades|StartCameraFade (Game|GetPlayerCameraManager 0) 0.0 1.0 (Variables|Default|GetDurationTime) "(R=0.000000,G=0.000000,B=0.000000,A=1.000000)" true false)
  (Utilities|FlowControl|Delay (Variables|Default|GetDurationTime))
  (bind _returnvalue (Game|GetCurrentLevelName true))
  (Game|OpenLevel(byName) (Utilities|String|StringToName _returnvalue)))

(event Custom|HitCrystal
  (Points|AddPoint))

(event Custom|Meta
  (params (Message :type Text) (TimeShowMessage :type Float%20%28single-precision%29))
  (Send|SendMessage Message)
  (Widget|SetVisibility (Variables|Default|GetHUD) "Visible")
  (Utilities|FlowControl|Delay TimeShowMessage)
  (Widget|SetVisibility (Variables|Default|GetHUD) "Hidden"))

(event EventBeginPlay
  (Points|SetMaxScore)
  (bind _returnvalue (UserInterface|CreateWidget "/Game/Wiget/UI_Messege.UI_Messege_C" (Game|GetPlayerController 0)))
  (bind _output_get (Variables|Default|SetHUD _returnvalue))
  (UserInterface|Viewport|AddtoViewport _output_get 0)
  (bind _returnvalue_2 (Game|GetCurrentLevelName true))
  (if (Utilities|Enum|Equal(Enum) _returnvalue_2 (Variables|Default|GetLevel_2))
    (CallFunction|SetCameraDistance 3e+01)))

(event Input|AxisEvents|InputAxisForwar|Back
  (params (AxisValue :type Float%20%28single-precision%29))
  ;[1 1 1] MoveBall
  (Class|PrimitiveComponent|AddTorqueinDegrees (Variables|Default|GetBall) (Math|Vector|MakeVector 0.0 (* AxisValue (Variables|Default|GetSpeedRotation)) 0.0) "None" true))

(event Input|AxisEvents|InputAxisLeft|Raight
  (params (AxisValue :type Float%20%28single-precision%29))
  ;[1 1 1] MoveBall
  (Class|PrimitiveComponent|AddTorqueinDegrees (Variables|Default|GetBall) (Math|Vector|MakeVector (* AxisValue (Variables|Default|GetSpeedRotation)) 0.0 0.0) "None" true))

(fn ConstructionScript)

(fn GetPlayerScore
  (return (Variables|Points|GetPoints)))

(fn AddPoint
  (Variables|Points|SetPoints (+ (Variables|Points|GetPoints) 1)))

(fn GetMaxScore
  (return (Variables|Points|GetMaxScore)))

(fn SetMaxScore
  (bind _outactors (Actor|GetAllActorsOfClass "/Game/Blueprints/Actors/Cyrstal/BP_Crystal.BP_Crystal_C"))
  (Variables|Points|SetMaxScore (Utilities|Array|Length _outactors)))

(fn SendMessage
  (params (Message :type Text))
  (Default|SetMessage (Variables|Default|GetHUD) Message))

(fn SetCameraDistance
  (params (NewParam :type Float%20%28single-precision%29))
  (Variables|/Script/Engine.SpringArmComponent|SetTargetArmLength (Variables|Default|GetSpringArm) NewParam)
  (return))

(fn GetSpring
  (return (Variables|Default|GetSpringArm)))